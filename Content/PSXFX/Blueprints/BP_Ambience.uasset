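; PSXFX ambience actor that controls the global lighting, fog and dither post-process for PSX-style rendering.
; Construction and BeginPlay write light, shade, falloff and fog values to MPC_PSXFX, taking light direction from the negated actor forward vector.
; They also assign a dynamic legacy or newer post-process material that carries the dither limit.
; Setter functions update individual parameters at runtime, most clamping their input.
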(event EventBeginPlay
  (CallFunction|InitializeParameters))

(fn ConstructionScript
  (CallFunction|InitializeParameters))

(fn SetLightIntensity
  (params (Intensity :type Float%20%28single-precision%29))
  (bind _color (Variables|Settings|Lighting|GetColor))
  (bind _output_get (Variables|Settings|Lighting|SetIntensity (Math|Float|Max(Float) Intensity 0.0)))
  (Rendering|Material|SetVectorParameterValue "/Game/PSXFX/Materials/MPC_PSXFX.MPC_PSXFX" "Global Light Color" (Utilities|Struct|MakeLinearColor (.r _color) (.g _color) (.b _color) _output_get) :!class /Script/Engine.KismetMaterialLibrary)
  (return))

(fn SetLightColor
  (params (Color :type Linear%20Color%20Structure))
  (bind _output_get (Variables|Settings|Lighting|SetColor (Utilities|Struct|MakeLinearColor (Math|Float|Clamp(Float) (.r Color)) (Math|Float|Clamp(Float) (.g Color)) (Math|Float|Clamp(Float) (.b Color)) 1.0)))
  (Rendering|Material|SetVectorParameterValue "/Game/PSXFX/Materials/MPC_PSXFX.MPC_PSXFX" "Global Light Color" (Utilities|Struct|MakeLinearColor (.r _output_get) (.g _output_get) (.b _output_get) (Variables|Settings|Lighting|GetIntensity)) :!class /Script/Engine.KismetMaterialLibrary)
  (return))

(fn SetVertexNormalInfluence
  (params (Influence :type Float%20%28single-precision%29))
  (bind _output_get (Variables|Settings|Lighting|SetVertexNormalInfluence (Math|Float|Clamp(Float) Influence)))
  (Rendering|Material|SetScalarParameterValue "/Game/PSXFX/Materials/MPC_PSXFX.MPC_PSXFX" "Global Light Dot" _output_get :!class /Script/Engine.KismetMaterialLibrary)
  (return))

(fn SetLightRotation
  (params (Rotation :type Rotator))
  (Transformation|SetActorRotation Rotation)
  (Rendering|Material|SetVectorParameterValue "/Game/PSXFX/Materials/MPC_PSXFX.MPC_PSXFX" "Global Light Direction" (Math|Conversions|ToLinearColor(Vector) (Math|Vector|NegateVector (Transformation|GetActorForwardVector))) :!class /Script/Engine.KismetMaterialLibrary)
  (return))

(fn SetFogColor
  (params (Color :type Linear%20Color%20Structure))
  (bind _output_get (Variables|Settings|Fog|SetFogColor (Utilities|Struct|MakeLinearColor (Math|Float|Clamp(Float) (.r Color)) (Math|Float|Clamp(Float) (.g Color)) (Math|Float|Clamp(Float) (.b Color)) (Variables|Settings|Fog|GetFogDensity))))
  (Rendering|Material|SetVectorParameterValue "/Game/PSXFX/Materials/MPC_PSXFX.MPC_PSXFX" "Fog RGBA" _output_get :!class /Script/Engine.KismetMaterialLibrary)
  (return))

(fn SetFogDensity
  (params (Density :type Float%20%28single-precision%29))
  (bind _fogcolor (Variables|Settings|Fog|GetFogColor))
  (bind _output_get (Variables|Settings|Fog|SetFogDensity (Math|Float|Clamp(Float) Density)))
  (Rendering|Material|SetVectorParameterValue "/Game/PSXFX/Materials/MPC_PSXFX.MPC_PSXFX" "Fog RGBA" (Utilities|Struct|MakeLinearColor (.r _fogcolor) (.g _fogcolor) (.b _fogcolor) _output_get) :!class /Script/Engine.KismetMaterialLibrary)
  (return))

(fn SetFogStartDistance
  (params (FogStartDistance :type Float%20%28single-precision%29))
  (bind _output_get (Variables|Settings|Fog|SetFogStartDistance FogStartDistance))
  (Rendering|Material|SetScalarParameterValue "/Game/PSXFX/Materials/MPC_PSXFX.MPC_PSXFX" "Fog Start Distance" _output_get :!class /Script/Engine.KismetMaterialLibrary)
  (return))

(fn SetFogFadeLength
  (params (Length :type Float%20%28single-precision%29))
  (bind _output_get (Variables|Settings|Fog|SetFogFadeLength (Math|Float|Max(Float) Length 0.0)))
  (Rendering|Material|SetScalarParameterValue "/Game/PSXFX/Materials/MPC_PSXFX.MPC_PSXFX" "Fog Fade Length" _output_get :!class /Script/Engine.KismetMaterialLibrary)
  (return))

(fn SetFogHeightOffset
  (params (Offset :type Float%20%28single-precision%29))
  (bind _output_get (Variables|Settings|Fog|SetFogHeightOffset Offset))
  (Rendering|Material|SetScalarParameterValue "/Game/PSXFX/Materials/MPC_PSXFX.MPC_PSXFX" "Fog Height Offset" _output_get :!class /Script/Engine.KismetMaterialLibrary)
  (return))

(fn SetFogHeightFadeLength
  (params (Length :type Float%20%28single-precision%29))
  (bind _output_get (Variables|Settings|Fog|SetFogHeightFadeLength Length))
  (Rendering|Material|SetScalarParameterValue "/Game/PSXFX/Materials/MPC_PSXFX.MPC_PSXFX" "Fog Height Fade Length" _output_get :!class /Script/Engine.KismetMaterialLibrary)
  (return))

(fn SetDitherLimit
  (params (Limit :type Float%20%28single-precision%29))
  (bind _output_get (Variables|Settings|SetDitherLimit (Math|Float|Max(Float) Limit 0.0)))
  (Rendering|Material|SetScalarParameterValue (Variables|Default|GetMID_PostProcess) "Limit" _output_get :!class /Script/Engine.MaterialInstanceDynamic)
  (return))

(fn InitializeParameters
  (bind _fogcolor (Variables|Settings|Fog|GetFogColor))
  (bind _color (Variables|Settings|Lighting|GetColor))
  (Utilities|FlowControl|Sequence
    (:then_0
      (Rendering|Material|SetVectorParameterValue "/Game/PSXFX/Materials/MPC_PSXFX.MPC_PSXFX" "Global Light Direction" (Math|Conversions|ToLinearColor(Vector) (Math|Vector|NegateVector (Transformation|GetActorForwardVector))) :!class /Script/Engine.KismetMaterialLibrary)
      (Rendering|Material|SetVectorParameterValue "/Game/PSXFX/Materials/MPC_PSXFX.MPC_PSXFX" "Global Light Color" (Utilities|Struct|MakeLinearColor (.r _color) (.g _color) (.b _color) (Variables|Settings|Lighting|GetIntensity)) :!class /Script/Engine.KismetMaterialLibrary)
      (Rendering|Material|SetVectorParameterValue "/Game/PSXFX/Materials/MPC_PSXFX.MPC_PSXFX" "Global Shade Color" (Variables|Settings|Lighting|GetShadeColor) :!class /Script/Engine.KismetMaterialLibrary)
      (Rendering|Material|SetScalarParameterValue "/Game/PSXFX/Materials/MPC_PSXFX.MPC_PSXFX" "Global Light Dot" (Variables|Settings|Lighting|GetVertexNormalInfluence) :!class /Script/Engine.KismetMaterialLibrary)
      (Rendering|Material|SetScalarParameterValue "/Game/PSXFX/Materials/MPC_PSXFX.MPC_PSXFX" "Fog Start Distance" (Variables|Settings|Fog|GetFogStartDistance) :!class /Script/Engine.KismetMaterialLibrary)
      (Rendering|Material|SetScalarParameterValue "/Game/PSXFX/Materials/MPC_PSXFX.MPC_PSXFX" "Fog Fade Length" (Variables|Settings|Fog|GetFogFadeLength) :!class /Script/Engine.KismetMaterialLibrary)
      (Rendering|Material|SetScalarParameterValue "/Game/PSXFX/Materials/MPC_PSXFX.MPC_PSXFX" "Fog Height Offset" (Variables|Settings|Fog|GetFogHeightOffset) :!class /Script/Engine.KismetMaterialLibrary)
      (Rendering|Material|SetScalarParameterValue "/Game/PSXFX/Materials/MPC_PSXFX.MPC_PSXFX" "Fog Height Fade Length" (Variables|Settings|Fog|GetFogHeightFadeLength) :!class /Script/Engine.KismetMaterialLibrary)
      (Rendering|Material|SetVectorParameterValue "/Game/PSXFX/Materials/MPC_PSXFX.MPC_PSXFX" "Fog RGBA" (Utilities|Struct|MakeLinearColor (.r _fogcolor) (.g _fogcolor) (.b _fogcolor) (Variables|Settings|Fog|GetFogDensity)) :!class /Script/Engine.KismetMaterialLibrary)
      (Rendering|Material|SetScalarParameterValue "/Game/PSXFX/Materials/MPC_PSXFX.MPC_PSXFX" "Light Falloff" (Variables|Settings|Lighting|GetFalloff) :!class /Script/Engine.KismetMaterialLibrary)
      (bind _returnvalue (Rendering|Material|CreateDynamicMaterialInstance (select (Variables|Settings|GetUseLegacyPostProcess) "/Game/PSXFX/Materials/M_PostProcess.M_PostProcess" "/Game/PSXFX/Materials/M_PostProcess_2.M_PostProcess_2") "None" :!class /Script/Engine.KismetMaterialLibrary))
      (bind _output_get (Variables|Default|SetMID_PostProcess _returnvalue))
      (Utilities|Struct|SetmembersinPostProcessSettings (Variables|/Script/Engine.PostProcessComponent|GetSettings (Variables|Default|GetPostProcess)) (Utilities|Struct|MakeWeightedBlendables (Utilities|Array|MakeArray (Utilities|Struct|MakeWeightedBlendable 1.0 _output_get)))))
    (:then_1
      (bind _mid_postprocess (Variables|Default|GetMID_PostProcess)
        (:then
          (Rendering|Material|SetScalarParameterValue _mid_postprocess "Limit" (Variables|Settings|GetDitherLimit) :!class /Script/Engine.MaterialInstanceDynamic))
        (:else)))
    (:then_2
      (return))))

(fn SetGlobalShadeColor
  (params (Color :type Linear%20Color%20Structure%20%28by%20ref%29))
  (bind _output_get (Variables|Settings|Lighting|SetShadeColor Color))
  (Rendering|Material|SetVectorParameterValue "/Game/PSXFX/Materials/MPC_PSXFX.MPC_PSXFX" "Global Shade Color" _output_get :!class /Script/Engine.KismetMaterialLibrary)
  (return))

(fn GetShadeColor
  (return (Variables|Settings|Lighting|GetShadeColor)))

(fn SetLightFalloff
  (params (Falloff :type Float%20%28single-precision%29))
  (bind _output_get (Variables|Settings|Lighting|SetFalloff (Math|Float|Clamp(Float) Falloff)))
  (Rendering|Material|SetScalarParameterValue "/Game/PSXFX/Materials/MPC_PSXFX.MPC_PSXFX" "Light Falloff" _output_get :!class /Script/Engine.KismetMaterialLibrary)
  (return))

(fn GetLightFalloff
  (return (Variables|Settings|Lighting|GetFalloff)))