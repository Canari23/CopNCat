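; BP_Destructible is a data-asset-driven destructible actor that plays a material-driven explosion animation when it takes any damage.
; Construction sets the default mesh; damage enlarges its bounds, creates a dynamic material, spawns optional destroyed mesh, particles and sound, and can disable collision.
; A duration-scaled timeline feeds material Progress and directional Force (curve or constant), quantizing alpha to simulate a low framerate adjusted for time dilation.
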(event EventBeginPlay)

(event Game|Damage|EventAnyDamage
  (params (Damage :type Float%20%28single-precision%29) (DamageType :type Damage%20Type%20Object%20Reference) (InstigatedBy :type Controller%20Object%20Reference) (DamageCauser :type Actor%20Object%20Reference))
  (|Animation))

(fn ConstructionScript
  (Variables|Debug|SetRunConstructionScript false)
  (|BaseMeshSetup))

(fn InitializeAnimationData
  (bind _debugmessages (Variables|Configuration|GetDebugMessages))
  (bind _destructibledata (Variables|Configuration|GetDestructibleData))
  (bind _destructibledata_2 (Variables|Configuration|GetDestructibleData))
  (bind _debugmessages_2 (Variables|Configuration|GetDebugMessages))
  (bind _duration (Variables|/Game/PSXFX/Blueprints/BP_DestructibleData.BP_DestructibleData_C|GetDuration _destructibledata_2))
  (bind _returnvalue (/ 1.0 _duration))
  (bind _destructibledata_3 (Variables|Configuration|GetDestructibleData)
    (:then
      (bind _defaultmesh (Variables|/Game/PSXFX/Blueprints/BP_DestructibleData.BP_DestructibleData_C|GetDefaultMesh _destructibledata_3)
        (:then
          (bind _returnvalue_2 (Rendering|Material|CreateDynamicMaterialInstance (Variables|Default|GetStaticMesh) 0 (Rendering|Material|GetMaterial _defaultmesh 0) "None" :!class /Script/Engine.PrimitiveComponent))
          (Variables|Configuration|SetMID_Destructible _returnvalue_2)
          (Rendering|Material|SetScalarParameterValue (Variables|Configuration|GetMID_Destructible) "Rotation Rate" (Variables|/Game/PSXFX/Blueprints/BP_DestructibleData.BP_DestructibleData_C|GetPolygonRotationRate (Variables|Configuration|GetDestructibleData)) :!class /Script/Engine.MaterialInstanceDynamic)
          (Rendering|Material|SetScalarParameterValue (Variables|Configuration|GetMID_Destructible) "Blast Radius" (* (Variables|/Game/PSXFX/Blueprints/BP_DestructibleData.BP_DestructibleData_C|GetRadialForce _destructibledata) (Variables|/Game/PSXFX/Blueprints/BP_DestructibleData.BP_DestructibleData_C|GetDuration _destructibledata)) :!class /Script/Engine.MaterialInstanceDynamic)
          (Rendering|Material|SetVectorParameterValue (Variables|Configuration|GetMID_Destructible) "Direction" (Math|Conversions|ToLinearColor(Vector) (Math|Vector|Normalize (Variables|/Game/PSXFX/Blueprints/BP_DestructibleData.BP_DestructibleData_C|GetForceDirection (Variables|Configuration|GetDestructibleData)))) :!class /Script/Engine.MaterialInstanceDynamic)
          (Components|Timeline|SetPlayRate (Variables|Default|GetExplosion) _returnvalue)
          (Rendering|Material|SetScalarParameterValue (Variables|Configuration|GetMID_Destructible) "Framerate" (/ (Variables|/Game/PSXFX/Blueprints/BP_DestructibleData.BP_DestructibleData_C|GetFramerate _destructibledata_2) _returnvalue) :!class /Script/Engine.MaterialInstanceDynamic)
          (return))
        (:else
          (Development|PrintString "Error: Invalid default static mesh!" _debugmessages _debugmessages "(R=1.000000,G=0.021000,B=0.104000,A=1.000000)" 4.0)
          (return))))
    (:else
      (Development|PrintString "Error: Invalid destructible data asset!" _debugmessages_2 _debugmessages_2 "(R=1.000000,G=0.021000,B=0.104000,A=1.000000)" 4.0)
      (return))))

(fn ActivateEffects
  (bind _debugmessages (Variables|Configuration|GetDebugMessages))
  (Variables|Configuration|GetDestructibleData
    (:then
      (Development|PrintString "Hit")
      (Utilities|FlowControl|Sequence
        (:then_0
          (bind _destroyedmesh (Variables|/Game/PSXFX/Blueprints/BP_DestructibleData.BP_DestructibleData_C|GetDestroyedMesh (Variables|Configuration|GetDestructibleData))
            (:then
              (Variables|Default|GetDestroyedMesh
                (:then
                  _)
                (:else
                  (bind _returnvalue (AddComponent|AddStaticMeshComponent false)) ; Add destroyed mesh
                  (Variables|Default|SetDestroyedMesh _returnvalue)))
              (Components|StaticMesh|SetStaticMesh (Variables|Default|GetDestroyedMesh) _destroyedmesh))
            (:else)))
        (:then_1
          (Configuration|SetNewBoundsScale))
        (:then_2
          (bind _particlesystem (Variables|/Game/PSXFX/Blueprints/BP_DestructibleData.BP_DestructibleData_C|GetParticleSystem (Variables|Configuration|GetDestructibleData))
            (:then
              (bind _returnvalue_2 (AddComponent|AddParticleSystemComponent false (Math|Transform|MakeTransform (Variables|/Game/PSXFX/Blueprints/BP_DestructibleData.BP_DestructibleData_C|GetParticleRelativeLocation (Variables|Configuration|GetDestructibleData)) "0, 0, 0" "1,1,1")))
              (Effects|Components|ParticleSystem|SetTemplate _returnvalue_2 _particlesystem))
            (:else)))
        (:then_3
          (bind _sound (Variables|/Game/PSXFX/Blueprints/BP_DestructibleData.BP_DestructibleData_C|GetSound (Variables|Configuration|GetDestructibleData))
            (:then
              (Audio|SpawnSoundatLocation _sound (Transformation|GetActorLocation) "0, 0, 0" 1.0 1.0 0.0 0 0))
            (:else)))
        (:then_4
          (return))))
    (:else
      (Development|PrintString "Error: Invalid destructible data asset!" _debugmessages _debugmessages "(R=1.000000,G=0.021000,B=0.104000,A=1.000000)" 4.0)
      (return))))

(fn SetNewBoundsScale
  (bind _destructibledata (Variables|Configuration|GetDestructibleData))
  (bind _destructibledata_2 (Variables|Configuration|GetDestructibleData))
  (bind _destructibledata_3 (Variables|Configuration|GetDestructibleData)
    (:then
      (if (Variables|/Game/PSXFX/Blueprints/BP_DestructibleData.BP_DestructibleData_C|GetUseDirectionalForceCurve _destructibledata_3)
        (bind _directionalforcecurve (Variables|/Game/PSXFX/Blueprints/BP_DestructibleData.BP_DestructibleData_C|GetDirectionalForceCurve (Variables|Configuration|GetDestructibleData))
          (:then
            (Rendering|SetBoundsScale (Variables|Default|GetStaticMesh) (Math|Float|Max(Float) (/ (+ (* (Variables|/Game/PSXFX/Blueprints/BP_DestructibleData.BP_DestructibleData_C|GetRadialForce _destructibledata) (Variables|/Game/PSXFX/Blueprints/BP_DestructibleData.BP_DestructibleData_C|GetDuration _destructibledata)) (* (+ (Math|Float|Absolute(Float) (.MinValue (Class|CurveBase|GetValueRange _directionalforcecurve))) (.MaxValue (Class|CurveBase|GetValueRange _directionalforcecurve))) 2.0)) (.sphereradius (StaticMesh|GetBounds (Variables|/Script/Engine.StaticMeshComponent|GetStaticMesh (Variables|Default|GetStaticMesh))))) 2.0)))
          (:else
            (Rendering|SetBoundsScale (Variables|Default|GetStaticMesh) (Math|Float|Max(Float) (/ (* (+ (Variables|/Game/PSXFX/Blueprints/BP_DestructibleData.BP_DestructibleData_C|GetRadialForce _destructibledata_2) (Variables|/Game/PSXFX/Blueprints/BP_DestructibleData.BP_DestructibleData_C|GetConstantDirectionalForce _destructibledata_2)) (Variables|/Game/PSXFX/Blueprints/BP_DestructibleData.BP_DestructibleData_C|GetDuration _destructibledata_2)) (.sphereradius (StaticMesh|GetBounds (Variables|/Script/Engine.StaticMeshComponent|GetStaticMesh (Variables|Default|GetStaticMesh))))) 2.0) :!label _label)))
        (else
          (goto _label)))
      (return))
    (:else
      (return))))

(fn SimulateFramerate
  (params (Alpha :type Float%20%28single-precision%29))
  (bind _returnvalue (Class|GameplayStatics|GetGlobalTimeDilation))
  (bind _destructibledata (Variables|Configuration|GetDestructibleData))
  (bind _framerate (Variables|/Game/PSXFX/Blueprints/BP_DestructibleData.BP_DestructibleData_C|GetFramerate _destructibledata))
  (bind _duration (Variables|/Game/PSXFX/Blueprints/BP_DestructibleData.BP_DestructibleData_C|GetDuration _destructibledata))
  (bind _returnvalue_2 (* _framerate _duration))
  (bind _returnvalue_3 (/ _returnvalue_2 _returnvalue))
  (return (/ (Math|Conversions|ToFloat(Integer) (Math|Float|Floor (* Alpha _returnvalue_3))) _returnvalue_3)))

(fn UpdateMaterialParameters
  (params (Alpha :type Float%20%28single-precision%29))
  (bind _destructibledata (Variables|Configuration|GetDestructibleData))
  (bind _destructibledata_2 (Variables|Configuration|GetDestructibleData))
  (bind _directionalforcecurve (Variables|/Game/PSXFX/Blueprints/BP_DestructibleData.BP_DestructibleData_C|GetDirectionalForceCurve _destructibledata))
  (Rendering|Material|SetScalarParameterValue (Variables|Configuration|GetMID_Destructible) "Progress" Alpha :!class /Script/Engine.MaterialInstanceDynamic)
  (Utilities|IsValid _directionalforcecurve
    (:Is%20Valid
      (if (Variables|/Game/PSXFX/Blueprints/BP_DestructibleData.BP_DestructibleData_C|GetUseDirectionalForceCurve _destructibledata)
        (Rendering|Material|SetScalarParameterValue (Variables|Configuration|GetMID_Destructible) "Force" (* (Math|Curves|GetFloatValue _directionalforcecurve Alpha) (Variables|/Game/PSXFX/Blueprints/BP_DestructibleData.BP_DestructibleData_C|GetCurveMultiplier (Variables|Configuration|GetDestructibleData))) :!class /Script/Engine.MaterialInstanceDynamic)
        (else
          (Rendering|Material|SetScalarParameterValue (Variables|Configuration|GetMID_Destructible) "Force" (* Alpha (* (Variables|/Game/PSXFX/Blueprints/BP_DestructibleData.BP_DestructibleData_C|GetConstantDirectionalForce _destructibledata_2) (Variables|/Game/PSXFX/Blueprints/BP_DestructibleData.BP_DestructibleData_C|GetDuration _destructibledata_2))) :!class /Script/Engine.MaterialInstanceDynamic :!label _label))))
    (:Is%20Not%20Valid
      (goto _label)))
  (return))