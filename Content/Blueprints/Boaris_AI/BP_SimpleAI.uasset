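; Work-in-progress Boaris AI actor that loses health when the BP_Pounce character attacks it.
; A capsule overlap with an attacking BP_Pounce prints a debug message and subtracts Health, but reaching zero triggers nothing.
; Stun, caught-screen widget and death/destroy logic are disconnected, leaving the caught collision and Hit events without effect.
; TakeDamage spawns an emitter and plays the stun animation, but the event graph never calls it.
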(event OnComponentBeginOverlap(CaughtCollision)
  (params (OverlappedComponent :type Primitive%20Component%20Object%20Reference) (OtherActor :type Actor%20Object%20Reference) (OtherComp :type Primitive%20Component%20Object%20Reference) (OtherBodyIndex :type Integer) (bFromSweep :type Boolean) (SweepResult :type Hit%20Result%20Structure%20%28by%20ref%29))
  ;[1 1 1] re-connect when done
  (if (== (Utilities|GetClass OtherActor) "/Game/Blueprints/BP_Pounce.BP_Pounce_C")
    _))

(event OnComponentBeginOverlap(CapsuleComponent)
  (params (OverlappedComponent :type Primitive%20Component%20Object%20Reference) (OtherActor :type Actor%20Object%20Reference) (OtherComp :type Primitive%20Component%20Object%20Reference) (OtherBodyIndex :type Integer) (bFromSweep :type Boolean) (SweepResult :type Hit%20Result%20Structure%20%28by%20ref%29))
  ;[1 1 1] Take Damage
  (bind _asbp_pounce (Utilities|Casting|CastToBP_Pounce OtherActor))
  (if (Variables|/Game/Blueprints/BP_Pounce.BP_Pounce_C|GetAttack _asbp_pounce)
    (Development|PrintString "Hit with Tail")
    (bind _output_get (Variables|Default|SetHealth (- (Variables|Default|GetHealth) 0.25)))
    (if (<= _output_get 0.0)
      _)))

(event Collision|EventHit
  (params (MyComp :type Primitive%20Component%20Object%20Reference) (Other :type Actor%20Object%20Reference) (OtherComp :type Primitive%20Component%20Object%20Reference) (bSelfMoved :type Boolean) (HitLocation :type Vector :default "0, 0, 0") (HitNormal :type Vector :default "0, 0, 0") (NormalImpulse :type Vector :default "0, 0, 0") (Hit :type Hit%20Result%20Structure%20%28by%20ref%29))
  ;[1 1 1] Stun WIP
)

(fn ConstructionScript)

(fn TakeDamage
  (Effects|SpawnEmitteratLocation 0 (Transformation|GetActorLocation))
  (Components|Animation|PlayAnimation (Variables|Character|GetMesh) "/Game/Characters/Boaris/Animations/BoarisStunAnim_Anim.BoarisStunAnim_Anim" false))

(fn Death)