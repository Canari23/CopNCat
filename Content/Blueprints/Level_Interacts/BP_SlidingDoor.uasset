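; BP_SlidingDoor is a level interactable door that slides open once for the BP_Nyx actor.
; A Box overlap sets InZone when BP_Nyx enters, and any end overlap clears it.
; The MoveDoor event, not called within this graph, checks InZone and Opened, then plays a timeline that lerps InnerDoor's relative location.
; Opened is set during timeline updates, and nothing closes the door again.
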(event OnComponentBeginOverlap(Box)
  (params (OverlappedComponent :type Primitive%20Component%20Object%20Reference) (OtherActor :type Actor%20Object%20Reference) (OtherComp :type Primitive%20Component%20Object%20Reference) (OtherBodyIndex :type Integer) (bFromSweep :type Boolean) (SweepResult :type Hit%20Result%20Structure%20%28by%20ref%29))
  (if (== (Utilities|GetClass OtherActor) "/Game/Blueprints/BP_Nyx.BP_Nyx_C")
    (Variables|Default|SetInZone? true)))

(event OnComponentEndOverlap(Box)
  (params (OverlappedComponent :type Primitive%20Component%20Object%20Reference) (OtherActor :type Actor%20Object%20Reference) (OtherComp :type Primitive%20Component%20Object%20Reference) (OtherBodyIndex :type Integer))
  (Variables|Default|SetInZone? false))

(event Custom|MoveDoor
  (if (Variables|Default|GetInZone?)
    (if (not (Variables|Default|GetOpened?))
      (Variables|Default|SetInZone? false)
      (bind _newtrack_1 (Timeline|Timeline_0 PlayFromStart)
        (:Update
          (Transformation|SetRelativeLocation (Variables|Default|GetInnerDoor) (Math|Vector|Lerp(Vector) "10.000000,1.734827,80.000000" "-200.000000,1.734827,80.000000" _newtrack_1) false false)
          (Variables|Default|SetOpened? true))))))

(event EventBeginPlay)

(event Collision|EventActorBeginOverlap
  (params (OtherActor :type Actor%20Object%20Reference)))

(event EventTick
  (params (DeltaSeconds :type Float%20%28single-precision%29)))

(fn ConstructionScript)