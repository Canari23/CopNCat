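; Motorcycle movement component that drives its owning Pawn's physics-simulated capsule from movement input.
; Tick consumes normalized input and orients the capsule along its forward plus velocity, with up opposite GravityDirection.
; A looping 250 Hz timer runs FixedTick, which reseeds Velocity from the forward vector rather than physics velocity.
; It then adds custom gravity and input acceleration with planar damping, overwriting the body's linear velocity.
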(event Custom|FixedTick
  (Variables|NonEdit|SetVelocity (Math|Vector|GetForwardVector (Variables|Components|GetCollision)))
  (CallFunction|ApplyGravity true)
  (CallFunction|MovementVelocity (Variables|Edit|GetMax%20Speed) 6e+01)
  (Class|PrimitiveComponent|SetAllPhysicsLinearVelocity (Variables|Components|GetCollision) (Variables|NonEdit|GetVelocity) false))

(event EventBeginPlay
  (bind _aspawn (Utilities|Casting|CastToPawn (Components|GetOwner)))
  (bind _output_get (Variables|NonEdit|SetParentPawn _aspawn))
  (bind _ascapsule_collision (Utilities|Casting|CastToCapsuleComponent (Variables|/Script/Engine.Actor|GetRootComponent _output_get)))
  (Variables|Components|SetCollision _ascapsule_collision)
  (CallFunction|ConfigurePhysics)
  (bind _output_get_2 (Variables|NonEdit|SetDelta%20Time (/ (Math|Float|MakeLiteralFloat 1.0) (Math|Float|MakeLiteralFloat 2.5e+02))))
  (Utilities|Time|SetTimerbyFunctionName 0 "FixedTick" _output_get_2 true))

(event EventTick
  (params (DeltaSeconds :type Float%20%28single-precision%29))
  (bind _parentpawn (Variables|NonEdit|GetParentPawn)
    (:then
      (bind _returnvalue (Class|Pawn|ConsumeMovementInputVector _parentpawn))
      (Variables|NonEdit|SetInput (Math|Vector|Normalize _returnvalue))
      (bind _collision (Variables|Components|GetCollision)
        (:then
          (Transformation|SetWorldRotation _collision (Math|Rotator|MakeRotfromZX (Math|Vector|NegateVector (Variables|NonEdit|GetGravityDirection)) (Math|Vector|Normalize (+ (Math|Vector|GetForwardVector (Variables|Components|GetCollision)) (Variables|NonEdit|GetVelocity)))) false false))
        (:else)))
    (:else)))

(fn ConfigurePhysics
  (bind _collision (Variables|Components|GetCollision))
  (Components|Tick|SetTickGroup "TG_PostPhysics")
  (Physics|SetSimulatePhysics _collision true)
  (Physics|SetEnableGravity _collision true)
  (Collision|SetCollisionProfileName _collision "Pawn" true :!class /Script/Engine.PrimitiveComponent)
  (Class|PrimitiveComponent|SetPhysMaterialOverride _collision "/Game/Blueprints/Motorcycle/TirePhysicMat.TirePhysicMat"))

(fn ApplyGravity
  (params (GravityEnabled :type Boolean))
  (if GravityEnabled
    (Variables|NonEdit|SetVelocity (+ (Variables|NonEdit|GetVelocity) (* (* (Variables|NonEdit|GetGravityDirection) (Math|Float|MakeLiteralFloat 9.8e+02)) (Variables|NonEdit|GetDelta%20Time))))))

(fn MovementVelocity
  (params (MaxSpeed :type Float%20%28single-precision%29) (Acceleration :type Float%20%28single-precision%29))
  (Variables|NonEdit|SetVelocity (+ (* (- (* (* (Variables|NonEdit|GetInput) MaxSpeed) Acceleration) (* (Math|Vector|ProjectVectorontoPlane (Variables|NonEdit|GetVelocity) (Variables|NonEdit|GetGravityDirection)) Acceleration)) (Variables|NonEdit|GetDelta%20Time)) (Variables|NonEdit|GetVelocity))))