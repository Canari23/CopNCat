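; Security camera that sweeps its body on a looping or timed track and raises the alarm when it spots BP_Pounce.
; The CameraMovement timeline drives the body's yaw from BeginPlay.
; An AlarmTrigger overlap plays an alarm sound and reports a "Noise" event for AI hearing, unless PounceAbility is active.
; CamOff stops the sweep, hides the view shaft and disables the trigger collision.
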(event OnComponentBeginOverlap(AlarmTrigger)
  (params (OverlappedComponent :type Primitive%20Component%20Object%20Reference) (OtherActor :type Actor%20Object%20Reference) (OtherComp :type Primitive%20Component%20Object%20Reference) (OtherBodyIndex :type Integer) (bFromSweep :type Boolean) (SweepResult :type Hit%20Result%20Structure%20%28by%20ref%29))
  (bind _returnvalue (Transformation|GetActorLocation))
  (bind _asbp_pounce (Utilities|Casting|CastToBP_Pounce OtherActor))
  (if (not (Variables|/Game/Blueprints/BP_Pounce.BP_Pounce_C|GetPounceAbility _asbp_pounce))
    (Audio|PlaySoundatLocation "/Game/Blueprints/SecurityCam_AI/alarm_Cue.alarm_Cue" _returnvalue "0, 0, 0" 1.0 1.0 0.0 0 0 0)
    (Class|AISenseHearing|ReportNoiseEvent _returnvalue 1.0 self 0.0 "Noise")))

(event Custom|CamOff
  (Audio|Components|Audio|Stop (Variables|Default|GetcameraMovement))
  (Rendering|SetVisibility (Variables|Components|GetViewShaft) false false)
  (Collision|SetCollisionEnabled (Variables|Default|GetAlarmTrigger) "NoCollision"))

(event EventBeginPlay
  ;[1 1 1] SecCam Rotation
  (bind _rotation (Timeline|cameraMovement Play)
    (:Update
      (Transformation|SetRelativeRotation (Variables|Components|Getcam_body) (Math|Rotator|MakeRotator 45.0 0.0 _rotation) false false))))

(fn ConstructionScript)